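; CarController handles touch input, turning horizontal swipes into SwipeLeft and SwipeRight calls on the player's CarBase pawn.
; A press records the start position and enables a per-tick check against a 30-unit distance threshold using the stored end position.
; A DoOnce, reset on release, then samples the live touch position and picks a direction if horizontal movement dominates.
; IsPressed is never cleared, so checking continues after release.
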(event `self.ReceiveTick`
  (params (DeltaSeconds :type "Float (single-precision)"))
  (if (`self.IsPressed`)
    (`self.CheckSwiping`)))

(event `CheckSwiping`
  (bind (_locationx _locationy) (`self.GetInputTouchState` (`GameplayStatics.GetPlayerController` 0) "Touch1"))
  (bind (_x _y) (`KismetMathLibrary.BreakVector2D` (- (`self.StartTouchPosition`) (`self.EndTouchPosition`))))
  (if (> (`KismetMathLibrary.VSize2D` (- (`self.EndTouchPosition`) (`self.StartTouchPosition`))) 30.0)
    (`/Engine/EditorBlueprintResources/StandardMacros.DoOnce` false :!label _label
      (:`Completed`
        (set `self.EndTouchPosition` (`KismetMathLibrary.MakeVector2D` _locationx _locationy))
        (if (> (`KismetMathLibrary.Abs` _x) (`KismetMathLibrary.Abs` _y))
          ;[1 1 1] left\right
          (if (> _x 0.0)
            (bind _ascar_base (cast `/Game/Blueprints/Pawns/Base/CarBase` (`GameplayStatics.GetPlayerPawn` 0)))
            (`KismetSystemLibrary.PrintString` "left")
            (`/Game/Blueprints/Pawns/Cars/DefaultCar.SwipeLeft` _ascar_base)
            (else
              (bind _ascar_base_2 (cast `/Game/Blueprints/Pawns/Base/CarBase` (`GameplayStatics.GetPlayerPawn` 0)))
              (`KismetSystemLibrary.PrintString` "right")
              (`/Game/Blueprints/Pawns/Cars/DefaultCar.SwipeRight` _ascar_base_2))))))))

(event `InputTouch`
  (params (Location :type "Vector Structure") (FingerIndex :type "ETouchIndex Enum"))
  (bind _x (.x Location))
  (bind _y (.y Location))
  (:`Pressed`
    (set `self.IsPressed` true)
    (set `self.StartTouchPosition` (`KismetMathLibrary.MakeVector2D` _x _y)))
  (:`Released`
    (set `self.EndTouchPosition` (`KismetMathLibrary.MakeVector2D` _x _y))
    (goto _label :!via `Reset`)))

(fn `UserConstructionScript`)